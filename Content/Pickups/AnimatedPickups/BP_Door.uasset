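; Interactable colored door that, when unlocked, swings open and then closes itself after a short pause.
; A dot product of the player-to-door direction and the door's forward vector picks the swing direction from the player's side.
; The Alpha timeline lerps the Arrow component's yaw and plays in reverse to close.
; The construction script tints the Cube with PickupColor through a dynamic material instance.
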(event Custom|ReverseTimeline
  (bind (_direction _alpha) (Timeline|Alpha Reverse)
    (:Update
      (Transformation|SetRelativeRotation (Variables|Default|GetArrow) (Math|Rotator|MakeRotator 0.0 0.0 (Math|Float|Lerp 0.0 (* (stale EventINTInteract _returnvalue) -1.0) _alpha)) false false))
    (:Finished
      (if (Utilities|Enum|Equal(Enum) _direction "Forward")
        (Utilities|FlowControl|Delay 1.0)
        (CallFunction|ReverseTimeline)))))

(event EventINTInteract
  (params (PlayerRef :type Player%20Char%20BP%20Object%20Reference))
  (if (Variables|Default|GetIsUnlocked)
    (bind _returnvalue (CallFunction|UpdateDoorAngle PlayerRef))
    (bind (_direction _alpha) (Timeline|Alpha Play)
      (:Update
        (Transformation|SetRelativeRotation (Variables|Default|GetArrow) (Math|Rotator|MakeRotator 0.0 0.0 (Math|Float|Lerp 0.0 (* _returnvalue -1.0) _alpha)) false false))
      (:Finished
        (if (Utilities|Enum|Equal(Enum) _direction "Forward")
          (Utilities|FlowControl|Delay 1.0)
          (CallFunction|ReverseTimeline))))))

(fn ConstructionScript
  (bind _returnvalue (Rendering|Material|CreateDynamicMaterialInstance (Variables|Default|GetCube) 0 "/Game/Pickups/AnimatedPickups/MAT_Color/MAT_Color.MAT_Color" "None" :!class /Script/Engine.PrimitiveComponent))
  (bind _output_get (Variables|Default|SetColorDMI _returnvalue))
  (Rendering|Material|SetVectorParameterValue _output_get "Color" (Variables|Default|GetPickupColor) :!class /Script/Engine.MaterialInstanceDynamic))

(fn UpdateDoorAngle
  (params (self2 :type Actor%20Object%20Reference))
  (return (select (> (Math|Vector|DotProduct (Math|Vector|GetUnitDirection(Vector) (Transformation|GetActorLocation self2) (Transformation|GetActorLocation)) (Transformation|GetActorForwardVector)) 0.0) 9e+01 -9e+01)))