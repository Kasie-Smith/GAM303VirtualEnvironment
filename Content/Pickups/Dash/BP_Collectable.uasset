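; A collectable pickup that the player gathers by interacting while in range.
; Box overlap events set a CanCollect flag for PlayerChar_BP actors and store a reference to the player on entry.
; The Interact event checks that flag, increments the player's CollectibleCount and destroys the pickup, with debug prints along the way.
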(event OnComponentBeginOverlap(Box)
  (params (OverlappedComponent :type Primitive%20Component%20Object%20Reference) (OtherActor :type Actor%20Object%20Reference) (OtherComp :type Primitive%20Component%20Object%20Reference) (OtherBodyIndex :type Integer) (bFromSweep :type Boolean) (SweepResult :type Hit%20Result%20Structure%20%28by%20ref%29))
  (bind _asplayer_char_bp (Utilities|Casting|CastToPlayerChar_BP OtherActor))
  (Variables|Default|SetPlayerRef _asplayer_char_bp)
  (Variables|Default|SetCanCollect true)
  (Development|PrintString "IN RANGE"))

(event OnComponentEndOverlap(Box)
  (params (OverlappedComponent :type Primitive%20Component%20Object%20Reference) (OtherActor :type Actor%20Object%20Reference) (OtherComp :type Primitive%20Component%20Object%20Reference) (OtherBodyIndex :type Integer))
  (Utilities|Casting|CastToPlayerChar_BP OtherActor)
  (Variables|Default|SetCanCollect false))

(event EventInteract
  (bind _playerref (Variables|Default|GetPlayerRef))
  (Development|PrintString "INTERACT RECEIVED")
  (if (Variables|Default|GetCanCollect)
    (bind _output_get (Variables|/Game/Player/PlayerChar_BP.PlayerChar_BP_C|SetCollectibleCount _playerref (+ (Variables|/Game/Player/PlayerChar_BP.PlayerChar_BP_C|GetCollectibleCount _playerref) 1)))
    (Development|PrintString (Utilities|String|ToString(Integer) _output_get))
    (Actor|DestroyActor)))

(fn ConstructionScript
  (|CallParentFunction))