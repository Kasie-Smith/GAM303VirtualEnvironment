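; BP_PhysicsPickup is a physics cube pickup that the player can grab and drop through interface-style events.
; Interact, if the player holds nothing, sets IsHolding, disables physics and snaps the Cube to the player's HoldPoint.
; Drop calls DetachFromActor and re-enables physics, leaving IsHolding untouched.
; The construction script tints the Cube with PickupColor through a dynamic material instance.
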(event EventINTInteract
  (params (PlayerRef :type Player%20Char%20BP%20Object%20Reference))
  (bind _cube (Variables|Default|GetCube))
  ;[0.15 0.15 0.15 0.5] Grab/Drop
  (if (not (Variables|/Game/Player/PlayerChar_BP.PlayerChar_BP_C|GetIsHolding? PlayerRef))
    (Variables|/Game/Player/PlayerChar_BP.PlayerChar_BP_C|SetIsHolding? PlayerRef true)
    (Physics|SetSimulatePhysics _cube false)
    (Collision|SetCollisionEnabled _cube "QueryAndPhysics")
    (Transformation|AttachComponentToComponent (Variables|Default|GetCube) (Variables|/Game/Player/PlayerChar_BP.PlayerChar_BP_C|GetHoldPoint PlayerRef) "None" "SnapToTarget" "SnapToTarget" "KeepWorld" false)))

(event EventINTDrop
  (params (PlayerRef :type Player%20Char%20BP%20Object%20Reference))
  (bind _cube (Variables|Default|GetCube))
  ;[0.15 0.15 0.15 0.5] Grab/Drop
  (Transformation|DetachFromActor "KeepWorld" "KeepWorld" "KeepWorld")
  (Collision|SetCollisionEnabled _cube "QueryAndPhysics")
  (Physics|SetSimulatePhysics _cube true))

(fn ConstructionScript
  (bind _returnvalue (Rendering|Material|CreateDynamicMaterialInstance (Variables|Default|GetCube) 0 "/Game/Pickups/AnimatedPickups/MAT_Color/MAT_Color.MAT_Color" "None" :!class /Script/Engine.PrimitiveComponent))
  (bind _output_get (Variables|Default|SetColorDMI _returnvalue))
  (Rendering|Material|SetVectorParameterValue _output_get "Color" (Variables|Default|GetPickupColor) :!class /Script/Engine.MaterialInstanceDynamic))