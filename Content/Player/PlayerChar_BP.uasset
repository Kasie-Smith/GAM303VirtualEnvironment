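; Player character Blueprint that handles first-hand input for moving, looking, jumping and interacting, and tracks score and respawning.
; Interact line-traces from the camera and sends an interface message to the hit actor, or sends it a drop message when IsHolding is set.
; AddScore accumulates and prints the score, while Respawn resets health and teleports to a random spawn point.
; CheckHealth is an empty stub.
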(event Custom|AddScore
  (params (AddAmount :type Integer))
  ;[0.15 0.15 0.15 0.5] Score
  (bind _output_get (Variables|Default|SetScore (+ (Variables|Default|GetScore) AddAmount)))
  (Development|PrintString (Utilities|String|ToString(Integer) _output_get)))

(event Custom|Respawn
  (bind _spawnpoints (Variables|Default|GetSpawnPoints))
  ;[0.15 0.15 0.15 0.5] Respawn
  (Variables|Default|SetHealth 1e+02)
  (Transformation|SetActorLocation (Transformation|GetActorLocation (Utilities|Array|Get(acopy) _spawnpoints (Math|Random|RandomIntegerinRange 0 (- (Utilities|Array|Length _spawnpoints) 1)))) false true))

(event Input|EnhancedActionEvents|EnhancedInputActionInput_Movement
  (params (ActionValue :type Vector%202D%20Structure) (ElapsedSeconds :type Float%20%28double-precision%29) (TriggeredSeconds :type Float%20%28double-precision%29) (InputAction :type Input%20Action%20Object%20Reference :default "/Game/Input/Input_Movement.Input_Movement"))
  (bind _returnvalue (Pawn|GetControlRotation :!class /Script/Engine.Pawn))
  ;[0.15 0.15 0.15 0.5] Input
  (Pawn|Input|AddMovementInput (Math|Vector|GetRightVector (Math|Rotator|MakeRotator (.roll _returnvalue) 0.0 (.yaw _returnvalue))) (.x ActionValue) false)
  (Pawn|Input|AddMovementInput (Math|Vector|GetForwardVector (Math|Rotator|MakeRotator 0.0 0.0 (.yaw _returnvalue))) (.y ActionValue) false))

(event Input|EnhancedActionEvents|EnhancedInputActionInput_Look
  (params (ActionValue :type Vector%202D%20Structure) (ElapsedSeconds :type Float%20%28double-precision%29) (TriggeredSeconds :type Float%20%28double-precision%29) (InputAction :type Input%20Action%20Object%20Reference :default "/Game/Input/Input_Look.Input_Look"))
  ;[0.15 0.15 0.15 0.5] Input
  (Pawn|Input|AddControllerYawInput (.x ActionValue))
  (Pawn|Input|AddControllerPitchInput (.y ActionValue)))

(event Input|EnhancedActionEvents|EnhancedInputActionInput_Interact
  (params (ActionValue :type Boolean) (ElapsedSeconds :type Float%20%28double-precision%29) (TriggeredSeconds :type Float%20%28double-precision%29) (InputAction :type Input%20Action%20Object%20Reference :default "/Game/Input/Input_Interact.Input_Interact"))
  (bind _camera (Variables|Default|GetCamera))
  (bind _returnvalue (Transformation|GetWorldLocation _camera))
  ;[0.01577 0.1855 0.06829 0.5] Player Interaction
  (:Started
    (if (Variables|Default|GetIsHolding?)
      (Class|BPIInteract|INTDrop(Message) (Variables|Default|GetHit%20Actor))
      (Variables|Default|SetIsHolding? false)
      (else
        (bind (_outhit _returnvalue_2) (Collision|LineTraceByChannel _returnvalue (+ _returnvalue (* (Math|Vector|GetForwardVector _camera) 8e+02)) "TraceTypeQuery1" false 0 "ForDuration"))
        (if _returnvalue_2
          (Variables|Default|SetHit%20Actor (.HitActor (Collision|BreakHitResult _outhit)))
          (Class|BPIInteract|INTInteract(Message) (.HitActor (Collision|BreakHitResult _outhit)) self))))))

(event Input|EnhancedActionEvents|EnhancedInputActionInput_Jump
  (params (ActionValue :type Boolean) (ElapsedSeconds :type Float%20%28double-precision%29) (TriggeredSeconds :type Float%20%28double-precision%29) (InputAction :type Input%20Action%20Object%20Reference :default "/Game/Input/Input_Jump.Input_Jump"))
  ;[0.15 0.15 0.15 0.5] Input
  (:Started
    (Character|Jump))
  (:Canceled
    (Character|StopJumping)))

(fn ConstructionScript)

(fn CheckHealth)